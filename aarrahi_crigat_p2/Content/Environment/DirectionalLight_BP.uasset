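; DirectionalLight_BP is a directional light that continuously cycles between day and night colour and intensity.
; Every Tick eases both values toward the opposite state of IsNight with a fixed-alpha lerp, closing a tenth of the gap per frame, so speed depends on frame rate.
; CheckHasReachedIntensity flips IsNight once intensity nearly equals its target, reversing the fade; colour is not checked.
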(event `self.ReceiveTick`
  (params (DeltaSeconds :type "Float (single-precision)"))
  (bind _returnvalue (* 0.9 1.0))
  (if (`self.IsNight`)
    ;[0.1437 0.4778 1] Lerp to Day Colour
    (`self.GoToLightColour` _returnvalue (`self.DayColour`))
    ;[1 0.8918 0.5104] Lerp to Day Intensity
    (`self.GoToLightIntensity` _returnvalue (`self.DayIntensity`))
    (`self.CheckHasReachedIntensity` (`self.DayIntensity`))
    (else
      ;[0.3229 0.01754 0.1542] Lerp to Night Colour
      (`self.GoToLightColour` _returnvalue (`self.NightColour`))
      ;[0.1042 0.09289 0.05317] Lerp to Night Intensity
      (`self.GoToLightIntensity` _returnvalue (`self.NightIntensity`))
      (`self.CheckHasReachedIntensity` (`self.NightIntensity`) true))))

(fn `CheckHasReachedIntensity`
  (params (Intensity :type "Float (double-precision)") (SetNight :type Boolean))
  (if (`KismetMathLibrary.NearlyEqual_FloatFloat` Intensity (`self.CurrentIntensity`))
    (set `self.IsNight` SetNight)))

(fn `GoToLightColour`
  (params (Alpha :type "Float (single-precision)") (Colour :type "Color Structure"))
  (bind _output_get (set `self.CurrentColour` (`KismetMathLibrary.Conv_LinearColorToColor` (`KismetMathLibrary.LinearColorLerp` (`KismetMathLibrary.Conv_ColorToLinearColor` Colour) (`KismetMathLibrary.Conv_ColorToLinearColor` (`self.CurrentColour`)) Alpha))))
  (`LightComponent.SetLightColor` (`self.Changing_DirectionalLight`) (`KismetMathLibrary.Conv_ColorToLinearColor` _output_get) true))

(fn `GoToLightIntensity`
  (params (Alpha :type "Float (double-precision)") (Intensity :type "Float (double-precision)"))
  (bind _output_get (set `self.CurrentIntensity` (`KismetMathLibrary.Lerp` Intensity (`self.CurrentIntensity`) Alpha)))
  (`LightComponent.SetIntensity` (`self.Changing_DirectionalLight`) _output_get))

(fn `UserConstructionScript`)