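; BP_Button is a puzzle button that changes the colour of a linked light when the player activates it nearby.
; Overlap with BP_ThirdPersonCharacter toggles an InRange flag and prints an on-screen prompt to press F.
; The actor enables player input and uses a debug key F event to call ChangeColorLight on the Light reference with its Colour, printing a too-far message otherwise.
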(event Collision|EventActorEndOverlap
  (params (OtherActor :type Actor%20Object%20Reference))
  (Utilities|Casting|CastToBP_ThirdPersonCharacter OtherActor)
  (Variables|Default|SetinRange false))

(event EventBeginPlay
  (Input|EnableInput (Game|GetPlayerController 0)))

(event Collision|EventActorBeginOverlap
  (params (OtherActor :type Actor%20Object%20Reference))
  (Utilities|Casting|CastToBP_ThirdPersonCharacter OtherActor)
  (Variables|Default|SetinRange true)
  (Development|PrintString "PREM F PER ENCENDRE"))

(event Input|KeyboardEvents|DebugKeyF
  (params (Key :type Key%20Structure :default "None") (ActionValue :type Input%20Action%20Value%20Structure))
  (:Pressed
    (Utilities|IsValid (Variables|Default|Getlight)
      (:Is%20Valid
        (if (Variables|Default|GetinRange)
          (Default|ChangeColorLight (Variables|Default|Getlight) (Variables|Default|Getcolour))
          (Development|PrintString "COLOR CANVIAT")
          (else
            (Development|PrintString "Has premut el botó massa lluny" :!label _label))))
      (:Is%20Not%20Valid
        (goto _label)))))

(fn ConstructionScript)