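; BP_PuzzleController checks a three-button colour combination puzzle.
; UpdateCurrentColour caches each button's current colour A value, and UpdatePuzzle compares those values with per-button desired values.
; As wired, success requires all three values to differ from their desired values, and either outcome is only printed as a debug string.
; No graph here calls either function.
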(fn `UpdateCurrentColour`
  (`|ExecutionSequence`
    (:`then_0`
      (bind _currentcoloura (`/Game/Puzzle/Button/BP_Button.GetCurrentColourA` (`self.Button1`)))
      (set `self.CurrentColourA1` _currentcoloura))
    (:`then_1`
      (bind _currentcoloura_2 (`/Game/Puzzle/Button/BP_Button.GetCurrentColourA` (`self.Button2`)))
      (set `self.CurrentColourA2` _currentcoloura_2))
    (:`then_2`
      (bind _currentcoloura_3 (`/Game/Puzzle/Button/BP_Button.GetCurrentColourA` (`self.Button3`)))
      (set `self.CurrentColourA3` _currentcoloura_3))))

(fn `UpdatePuzzle`
  (if (and (== (not (`self.CurrentColourA1`)) (`self.Button1Desired`)) (== (not (`self.CurrentColourA2`)) (`self.Button2Desired`)) (== (not (`self.CurrentColourA3`)) (`self.Button3Desired`)))
    (`KismetSystemLibrary.PrintString` "WELL DONE!!!!!!!!!!!!!!!" true true (struct :`R` 0.207596 :`G` 1.0 :`B` 0.20669 :`A` 1.0) 5.0)
    (else
      (`KismetSystemLibrary.PrintString` "WRONG COMBINATION" true true (struct :`R` 1.0 :`G` 0.130208 :`B` 0.471346 :`A` 1.0)))))

(fn `UserConstructionScript`)